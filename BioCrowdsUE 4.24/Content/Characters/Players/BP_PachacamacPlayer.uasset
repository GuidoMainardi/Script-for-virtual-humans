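; BP_PachacamacPlayer is a player Blueprint that switches between fixed overview cameras and player view at clicked points of interest.
; N cycles through CameraActors tagged "Overview", cutting instantly from player mode and blending between cameras otherwise.
; Left-clicking an actor whose first tag is "POI" moves the character there, blends the view to it, then enters player mode after a delay.
; The mode flag controls cursor visibility, and Escape quits.
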(event `self.ReceiveBeginPlay`
  (bind _outactors (`GameplayStatics.GetAllActorsOfClassWithTag` "/Script/Engine.CameraActor" "Overview"))
  (set `self.NumCameras` (`KismetArrayLibrary.Array_Length` _outactors))
  (set `self.CurrentCamera` 0))

(event `Key|N`
  (params (Key :type "Key Structure"))
  (:`Pressed`
    (bind _outactors (`GameplayStatics.GetAllActorsOfClassWithTag` "/Script/Engine.CameraActor" "Overview"))
    (if (`self.PlayerMode`)
      (set `self.BlendTime` 0.0)
      (else
        (bind _output_get (set `self.BlendTime` 2.0))))
    (`self.SetViewTargetWithBlend` (`GameplayStatics.GetPlayerController` 0) (`|GetArrayItem` _outactors (`self.CurrentCamera`)) _output_get "VTBlend_Linear" 0.0 false)
    (`KismetSystemLibrary.PrintString` (`KismetSystemLibrary.GetDisplayName` null))
    (set `self.CurrentCamera` (mod (+ (`self.CurrentCamera`) 1) (`self.NumCameras`)))
    (set `self.PlayerMode` false)
    (`self.UpdateCursor`)))

(event `Key|LeftMouseButton`
  (params (Key :type "Key Structure"))
  (bind _returnvalue (`GameplayStatics.GetPlayerCharacter` 0))
  (bind (_bblockinghit _binitialoverlap _time _distance _location _impactpoint _normal _impactnormal _physmat _hitactor) (`GameplayStatics.BreakHitResult` (`self.GetHitResultUnderCursorByChannel` (`GameplayStatics.GetPlayerController` 0) "TraceTypeQuery1" true)))
  (bind _returnvalue_2 (`self.K2_GetActorLocation` _hitactor))
  (:`Pressed`
    (if _bblockinghit
      (`KismetSystemLibrary.PrintString` (`KismetStringLibrary.Concat_StrStr` (`KismetStringLibrary.Concat_StrStr` (`KismetSystemLibrary.GetDisplayName` _hitactor) "\" \"") (`KismetStringLibrary.Conv_VectorToString` _returnvalue_2)))
      (if (== (`|GetArrayItem` (`Actor.Tags` _hitactor)) "POI")
        (`self.K2_SetActorLocation` _returnvalue _returnvalue_2 false false)
        (`self.SetViewTargetWithBlend` (`GameplayStatics.GetPlayerController` 0) _returnvalue 2.0 "VTBlend_Linear" 0.0 false)
        (`KismetSystemLibrary.Delay` 2.0)
        (set `self.PlayerMode` true)
        (`self.UpdateCursor`)))))

(event `Key|Escape`
  (params (Key :type "Key Structure"))
  (:`Pressed`
    (`KismetSystemLibrary.QuitGame` null "Quit")))

(fn `UpdateCursor`
  (set `PlayerController.bShowMouseCursor` (not (`self.PlayerMode`)) (`GameplayStatics.GetPlayerController` 0)))

(fn `UserConstructionScript`)