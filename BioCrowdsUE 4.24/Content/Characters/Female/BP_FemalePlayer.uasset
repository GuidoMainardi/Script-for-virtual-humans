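; BP_FemalePlayer is the female player character, with axis-driven look and movement relative to the control rotation's yaw.
; Keys 1 and 3 switch between a zero-length, first-person-style camera and a third-person one by setting the spring arm length.
; A SetSpeed function exposes the character's max walk speed, and leftover debug prints for animation speed and velocity are disconnected.
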(event `InputAxis|Turn`
  (params (AxisValue :type "Float (single-precision)"))
  (`self.AddControllerYawInput` AxisValue))

(event `InputAxis|LookUp`
  (params (AxisValue :type "Float (single-precision)"))
  (`self.AddControllerPitchInput` AxisValue))

(event `InputAxis|MoveForward`
  (params (AxisValue :type "Float (single-precision)"))
  (`self.AddMovementInput` (`KismetMathLibrary.GetForwardVector` (`KismetMathLibrary.MakeRotator` 0.0 0.0 (.yaw (`self.GetControlRotation`)))) AxisValue))

(event `InputAxis|MoveRight`
  (params (AxisValue :type "Float (single-precision)"))
  (`self.AddMovementInput` (`KismetMathLibrary.GetRightVector` (`KismetMathLibrary.MakeRotator` 0.0 0.0 (.yaw (`self.GetControlRotation`)))) AxisValue))

(event `self.ReceiveTick`
  (params (DeltaSeconds :type "Float (single-precision)")))

(event `Key|One`
  (params (Key :type "Key Structure"))
  (:`Pressed`
    (set `SpringArmComponent.TargetArmLength` 0.0 (`self.SpringArm`))))

(event `Key|Three`
  (params (Key :type "Key Structure"))
  (:`Pressed`
    (set `SpringArmComponent.TargetArmLength` 300.0 (`self.SpringArm`))))

(fn `SetSpeed`
  (params (Speed :type "Float (double-precision)"))
  (set `CharacterMovementComponent.MaxWalkSpeed` Speed (`self.CharacterMovement`)))

(fn `UserConstructionScript`)